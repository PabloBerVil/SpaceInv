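; BP_Enemy0 is an enemy actor that ends the game in failure when its hitbox overlaps a BP_TopDownCollider.
; SetSprite shows the enemy type by switching on a scalar parameter in a dynamic material instance.
; EnemyMove takes fixed steps along X or Y based on DirectionToMove.
; Despawning resets and hides the actor rather than destroying it, updating the scene manager's death count, enemy list and movement index.
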(event OnComponentBeginOverlap(Hitbox)
  (params (OverlappedComponent :type Primitive%20Component%20Object%20Reference) (OtherActor :type Actor%20Object%20Reference) (OtherComp :type Primitive%20Component%20Object%20Reference) (OtherBodyIndex :type Integer) (bFromSweep :type Boolean) (SweepResult :type Hit%20Result%20Structure%20%28by%20ref%29))
  (Utilities|Casting|CastToBP_TopDownCollider OtherActor)
  (Default|EndGameFailure (Variables|Default|GetSceneManagerRef)))

(fn ConstructionScript
  (|CallParentFunction))

(fn SetSprite
  ;[1 1 1] asigns a material instance and changes the texture to match the correct type of enemy in the material
  (if (Utilities|IsValid (Variables|Default|GetMaterialInst))
    _
    (else
      (bind _returnvalue (Rendering|Material|CreateDynamicMaterialInstance (Utilities|Array|Get(acopy) (Rendering|Material|GetMaterials (Variables|Default|GetSprite))) "None" "None" :!class /Script/Engine.KismetMaterialLibrary))
      (bind _output_get (Variables|Default|SetMaterialInst _returnvalue))
      (Rendering|Material|SetMaterial (Variables|Default|GetSprite) 0 _output_get)))
  (for (_array_element _array_index) (Variables|Default|GetParamNames)
    (if (== _array_index (Variables|Default|GetTypeOfEnemy))
      (Rendering|Material|SetScalarParameterValue (Variables|Default|GetMaterialInst) _array_element 1.0 :!class /Script/Engine.MaterialInstanceDynamic))))

(fn SetValuesonDespawn
  (bind _scenemanagerref (Variables|Default|GetSceneManagerRef))
  (bind _scenemanagerref_2 (Variables|Default|GetSceneManagerRef))
  (for _array_element (Variables|Default|GetParamNames)
    (Rendering|Material|SetScalarParameterValue (Variables|Default|GetMaterialInst) _array_element 0.0 :!class /Script/Engine.MaterialInstanceDynamic))
  (Variables|/Script/Engine.PrimitiveComponent|SetbGenerateOverlapEvents (Variables|Default|GetHitbox) false)
  (Variables|Default|SetIsAlive false)
  (Variables|/Game/MainFolder/Blueprints/Manager/SceneManager.SceneManager_C|SetDeadEnemiesNum _scenemanagerref (+ (Variables|/Game/MainFolder/Blueprints/Manager/SceneManager.SceneManager_C|GetDeadEnemiesNum _scenemanagerref) 1))
  (bind (_array_element_2 _array_index) (Utilities|Array|ForEachLoopwithBreak (Variables|/Game/MainFolder/Blueprints/Manager/SceneManager.SceneManager_C|GetNormalEnemiesList (Variables|Default|GetSceneManagerRef)) :!label _label)
    (:LoopBody
      (if (== _array_element_2 self)
        (if (<= _array_index (Variables|/Game/MainFolder/Blueprints/Manager/SceneManager.SceneManager_C|GetEnemyToAllowMove _scenemanagerref_2))
          (Variables|/Game/MainFolder/Blueprints/Manager/SceneManager.SceneManager_C|SetEnemyToAllowMove _scenemanagerref_2 (- (Variables|/Game/MainFolder/Blueprints/Manager/SceneManager.SceneManager_C|GetEnemyToAllowMove _scenemanagerref_2) 1)))
        (Utilities|Array|RemoveIndex (Variables|/Game/MainFolder/Blueprints/Manager/SceneManager.SceneManager_C|GetNormalEnemiesList _scenemanagerref_2) _array_index)
        (goto _label Break)))
    (:Completed
      (Rendering|SetActorHiddenInGame true))))

(fn EnemyMove
  (bind _returnvalue (Transformation|GetActorLocation))
  (bind _returnvalue_2 (Transformation|GetActorLocation))
  (bind _returnvalue_3 (Transformation|GetActorLocation))
  (bind _returnvalue_4 (Transformation|GetActorLocation))
  (switch int (Variables|Default|GetDirectionToMove)
    (:0
      (Transformation|SetActorLocation (Math|Vector|MakeVector (.x _returnvalue) (- (.y _returnvalue) 1e+01) (.z _returnvalue)) false false))
    (:1
      (Transformation|SetActorLocation (Math|Vector|MakeVector (- (.x _returnvalue_4) 1e+01) (.y _returnvalue_4) (.z _returnvalue_4)) false false))
    (:2
      (Transformation|SetActorLocation (Math|Vector|MakeVector (- (.x _returnvalue_2) 1e+01) (.y _returnvalue_2) (.z _returnvalue_2)) false false))
    (:3
      (Transformation|SetActorLocation (Math|Vector|MakeVector (.x _returnvalue_3) (+ (.y _returnvalue_3) 1e+01) (.z _returnvalue_3)) false false))))