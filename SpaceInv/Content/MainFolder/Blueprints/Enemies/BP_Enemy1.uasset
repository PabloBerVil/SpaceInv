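; BP_Enemy1 is an enemy Blueprint that moves with a ProjectileMovement component and deactivates itself after passing a left-side limit.
; Each tick it compares its Y location to LimitLeftToDespawn and calls SetValuesOnDespawn once at or below it.
; That function disables hitbox overlaps, zeroes velocity, hides the actor and stops its tick, leaving it dormant instead of destroyed.
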(event EventTick
  (params (DeltaSeconds :type Float%20%28single-precision%29))
  (if (<= (.y (Transformation|GetActorLocation)) (Variables|Default|GetLimitLeftToDespawn))
    (CallFunction|SetValuesonDespawn)))

(fn ConstructionScript
  (|CallParentFunction))

(fn SetValuesonDespawn
  (Variables|/Script/Engine.PrimitiveComponent|SetbGenerateOverlapEvents (Variables|Default|GetHitbox) false)
  (Variables|/Script/Engine.MovementComponent|SetVelocity (Variables|Default|GetProjectileMovement) "0, 0, 0")
  (Rendering|SetActorHiddenInGame true)
  (Actor|Tick|SetActorTickEnabled false))