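; Scene manager for a Space Invaders-style stage that spawns the player, orthographic camera, obstacles and enemy grid, then runs the wave until success or failure.
; An expandable actor pool supplies enemies, bullets and the periodic special enemy.
; Looping timers move one enemy per tick, turning the formation at side limits, and fire from a random column's bottom enemy.
; Each detected death shortens movement and shooting intervals and checks for victory.
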(event Custom|StartGame
  ;[1 1 1] Set the logic with timers and abilitates controls after a short initial delay
  (bind _output_get (Variables|Default|SetCurrentEnemySpeed (Variables|EnemySettings|GetMinEnemySpeed)))
  (bind _returnvalue (Utilities|Time|SetTimerbyFunctionName 0 "EnemyMove" _output_get true 1.7))
  (Variables|Default|SetSpeedTimer _returnvalue)
  (Utilities|FlowControl|Delay 1.7)
  (bind _asbp_player_controller (Utilities|Casting|CastToBP_PlayerController (Game|GetPlayerController 0)))
  (Variables|/Game/MainFolder/Blueprints/Player/BP_PlayerController.BP_PlayerController_C|SetEnabledInput _asbp_player_controller true)
  (bind _returnvalue_2 (Utilities|Time|SetTimerbyFunctionName 0 "SpawnSpecialEnemy" 2e+01 true))
  (Variables|Default|SetSpecialEnemSpawnTimer _returnvalue_2)
  (bind _output_get_2 (Variables|Default|SetCurrentEnemyShootFreq (Variables|EnemySettings|GetEnemyBaseShootFreq)))
  (bind _returnvalue_3 (Utilities|Time|SetTimerbyFunctionName 0 "EnemyShooting" _output_get_2 true 1.7))
  (Variables|Default|SetEnemyShootingTimer _returnvalue_3))

(event EventBeginPlay
  (bind _asbp_game_mode (Utilities|Casting|CastToBP_GameMode (Game|GetGameMode)))
  (Variables|/Game/MainFolder/Blueprints/Manager/BP_GameMode.BP_GameMode_C|SetSceneManagerRef _asbp_game_mode self)
  (MapSettings|InitialSettings))

(fn ConstructionScript)

(fn InitialSettings
  (PlayerSettings|SpawnPlayer)
  (MapSettings|SpawnCamera)
  (MapSettings|SpawnObstacles)
  (EnemySettings|SpawnEnemies))

(fn SpawnPlayer
  (bind _returnvalue (Game|GetPlayerController 0))
  (bind _returnvalue_2 (Game|SpawnActorfromClass "/Game/MainFolder/Blueprints/Player/BP_Player.BP_Player_C" (Math|Conversions|ToTransform(Vector) (Variables|PlayerSettings|GetPlayerPos)) "Undefined" 0 0))
  (Pawn|Possess _returnvalue _returnvalue_2)
  (bind _asbp_player_controller (Utilities|Casting|CastToBP_PlayerController _returnvalue))
  (Variables|/Game/MainFolder/Blueprints/Player/BP_PlayerController.BP_PlayerController_C|SetPlayerPawn _asbp_player_controller (Pawn|GetControlledPawn _asbp_player_controller))
  (Variables|/Game/MainFolder/Blueprints/Player/BP_PlayerController.BP_PlayerController_C|SetVelocity _asbp_player_controller (Variables|PlayerSettings|GetPlayerVelocity))
  (Variables|/Game/MainFolder/Blueprints/Player/BP_PlayerController.BP_PlayerController_C|SetLimitLeft _asbp_player_controller (Variables|MapSettings|GetLimitLeft))
  (Variables|/Game/MainFolder/Blueprints/Player/BP_PlayerController.BP_PlayerController_C|SetLimitRight _asbp_player_controller (Variables|MapSettings|GetLimitRight))
  (bind _asbp_player (Utilities|Casting|CastToBP_Player (Game|Player|GetPlayerPawn 0)))
  (Variables|/Game/MainFolder/Blueprints/Player/BP_Player.BP_Player_C|SetSceneManagerRef _asbp_player self))

(fn SpawnCamera
  (bind _returnvalue (Game|SpawnActorfromClass "/Script/Engine.CameraActor" (Variables|MapSettings|GetCameraPos) "Undefined" 0 0))
  (bind _output_get (Variables|Default|SetCameraRef _returnvalue))
  (Class|CameraComponent|SetProjectionMode (Variables|/Script/Engine.CameraActor|GetCameraComponent _output_get) "Orthographic")
  (Class|CameraComponent|SetOrthoWidth (Variables|/Script/Engine.CameraActor|GetCameraComponent _output_get) (Variables|MapSettings|GetCameraSize))
  (Game|Player|SetViewTargetwithBlend (Game|GetPlayerController 0) (Variables|Default|GetCameraRef) 0.0 "VTBlend_Linear" 0.0 false))

(fn SpawnObstacles
  (for _array_element (Variables|MapSettings|GetObstaclesNum)
    (Game|SpawnActorfromClass "/Game/MainFolder/Blueprints/Hazards/BP_Obstacle.BP_Obstacle_C" (Math|Transform|MakeTransform _array_element "0, 0, 0" "0.250000,0.250000,1") "Undefined" 0 0))
  (for _array_element_2 (Variables|MapSettings|GetTopDownColliders)
    (Game|SpawnActorfromClass "/Game/MainFolder/Blueprints/Hazards/BP_TopDownCollider.BP_TopDownCollider_C" (Math|Transform|MakeTransform (Math|Vector|MakeVector _array_element_2 0.0 0.0) "0, 0, 0" "1,1,1") "Undefined" 0 0)))

(fn ObjectPoolStart
  (for _array_element (Variables|ObjectPooler|GetObjectToPool)
    (bind _returnvalue (Game|SpawnActorfromClass _array_element (Variables|Default|GetPooledObjectLocat) "Undefined" 0 0))
    (Rendering|SetActorHiddenInGame _returnvalue true)
    (Utilities|Array|Add (Variables|ObjectPooler|GetPool) _returnvalue)))

(fn ObjectPoolSpawn
  (params (ActorType :type Actor%20Class%20Reference))
  (LocalVariables|SetActorClas ActorType)
  (for _array_element (Variables|ObjectPooler|GetPool)
    ;[1 1 1] obtains an matching actor from the pool
    (bind _output_get (LocalVariables|SetActorRefe _array_element))
    (if (== (Utilities|GetClass _output_get) (LocalVariables|GetActorClas))
      (if (Variables|/Script/Engine.Actor|GetbHidden (LocalVariables|GetActorRefe))
        (return (LocalVariables|GetActorRefe)))))
  ;[1 1 1] adds an actor to the pool if there is none disponible before returning an actor
  (bind _returnvalue (Game|SpawnActorfromClass (LocalVariables|GetActorClas) (Variables|Default|GetPooledObjectLocat) "Undefined" 0 0))
  (Utilities|Array|Add (Variables|ObjectPooler|GetPool) _returnvalue)
  (Rendering|SetActorHiddenInGame _returnvalue true)
  (return _returnvalue))

(fn SpawnEnemies
  ;[1 1 1] for each row of enemies, it spawns the correct class´ one and sets its variables (position, sprite...). Then adds it to a list of enemies. Then sets to a list enemies prepared to shoot depending of the number of columns of enemies
  (for (_array_element _array_index) (Variables|EnemySettings|GetEnemyRows)
    (for (_array_element_2 _array_index_2) (.EnemyArray (Utilities|Struct|BreakSt_EnemyRow _array_element))
      (bind _actorref (ObjectPooler|ObjectPoolSpawn (.TypeOfEnemyClass (Utilities|Struct|BreakSt_EnemySlot _array_element_2))))
      (bind _asbp_enemy_0 (Utilities|Casting|CastToBP_Enemy0 _actorref)
        (:then
          (LocalVariables|SetSpawningEnem _asbp_enemy_0)
          (Transformation|SetActorLocation (LocalVariables|GetSpawningEnem) (Math|Vector|MakeVector (.x (.PositionOfRow (Utilities|Struct|BreakSt_EnemyRow _array_element))) (+ (/ (Math|Float|Absolute(Float) (- (Variables|MapSettings|GetLimitLeft) (Variables|MapSettings|GetLimitRight))) (Math|Conversions|ToFloat(Integer) (+ (Utilities|Array|Length (.EnemyArray (Utilities|Struct|BreakSt_EnemyRow _array_element))) 1))) (+ (* _array_index_2 (/ (Math|Float|Absolute(Float) (- (Variables|MapSettings|GetLimitLeft) (Variables|MapSettings|GetLimitRight))) (Math|Conversions|ToFloat(Integer) (+ (Utilities|Array|Length (.EnemyArray (Utilities|Struct|BreakSt_EnemyRow _array_element))) 1)))) (Variables|MapSettings|GetLimitLeft))) 0.0) false false)
          (Variables|/Game/MainFolder/Blueprints/Enemies/BP_EnemyBase.BP_EnemyBase_C|SetTypeOfEnemy (LocalVariables|GetSpawningEnem) (.TypeOfEnemy (Utilities|Struct|BreakSt_EnemySlot _array_element_2)))
          (Default|SetSprite (LocalVariables|GetSpawningEnem))
          (Variables|/Game/MainFolder/Blueprints/Enemies/BP_Enemy0.BP_Enemy0_C|SetAwardedPoints (LocalVariables|GetSpawningEnem) (- (Utilities|Array|Length (Variables|EnemySettings|GetEnemyRows)) _array_index))
          (Variables|/Game/MainFolder/Blueprints/Enemies/BP_EnemyBase.BP_EnemyBase_C|SetIsAlive (LocalVariables|GetSpawningEnem) true)
          (Variables|/Script/Engine.PrimitiveComponent|SetbGenerateOverlapEvents (Variables|/Game/MainFolder/Blueprints/Enemies/BP_EnemyBase.BP_EnemyBase_C|GetHitbox (LocalVariables|GetSpawningEnem)) true)
          (Variables|/Game/MainFolder/Blueprints/Enemies/BP_EnemyBase.BP_EnemyBase_C|SetSceneManagerRef (LocalVariables|GetSpawningEnem) self)
          (Variables|/Game/MainFolder/Blueprints/Enemies/BP_Enemy0.BP_Enemy0_C|SetRow (LocalVariables|GetSpawningEnem) _array_index)
          (Variables|/Game/MainFolder/Blueprints/Enemies/BP_Enemy0.BP_Enemy0_C|SetColumn (LocalVariables|GetSpawningEnem) _array_index_2)
          (Utilities|Array|Add (Variables|Default|GetNormalEnemiesList) (LocalVariables|GetSpawningEnem))
          (bind _returnvalue (Game|SpawnActorfromClass "/Game/MainFolder/Blueprints/Enemies/BP_AIController.BP_AIController_C" (Math|Transform|MakeTransform "0, 0, 0" "0, 0, 0" "1,1,1") "Undefined" 0 0))
          (Pawn|Possess _returnvalue (LocalVariables|GetSpawningEnem))
          (Rendering|SetActorHiddenInGame (LocalVariables|GetSpawningEnem) false))
        (:CastFailed
          (Development|PrintString "Special enemy")))))
  (bind _output_get (Variables|Default|SetInitNumEnemies (Utilities|Array|Length (Variables|Default|GetNormalEnemiesList))))
  (Variables|Default|SetEnemyToAllowMove (- _output_get 1))
  (for _array_element_3 (Variables|EnemySettings|GetEnemyRows)
    (if (> (Utilities|Array|Length (.EnemyArray (Utilities|Struct|BreakSt_EnemyRow _array_element_3))) (Utilities|Array|Length (Variables|Default|GetEnemiesToShoot)))
      (for _array_element_4 (.EnemyArray (Utilities|Struct|BreakSt_EnemyRow _array_element_3))
        (if (> (Utilities|Array|Length (.EnemyArray (Utilities|Struct|BreakSt_EnemyRow _array_element_3))) (Utilities|Array|Length (Variables|Default|GetEnemiesToShoot)))
          (Utilities|Array|Add (Variables|Default|GetEnemiesToShoot) 0))))))

(fn MovebyTurn
  (bind _normalenemieslist (Variables|Default|GetNormalEnemiesList))
  (if (Utilities|IsValid (Utilities|Array|Get(acopy) _normalenemieslist (Variables|Default|GetEnemyToAllowMove)))
    (Default|EnemyMove (Utilities|Array|Get(acopy) _normalenemieslist (Variables|Default|GetEnemyToAllowMove))))
  (if (<= (Variables|Default|GetEnemyToAllowMove) 0)
    (Variables|Default|SetEnemyToAllowMove (- (Utilities|Array|Length _normalenemieslist) 1))
    (Variables|Default|SetChangeDirection true)
    (else
      (Variables|Default|SetEnemyToAllowMove (- (Variables|Default|GetEnemyToAllowMove) 1)))))

(fn EnemyChangeDirection
  ;[1 1 1] Change direction when someone has reached a limit or if the last move was down, directions are: 0-left, 1-downleft, 2-downright, 3-right
  (Variables|Default|SetChangeDirection false)
  (switch int (Variables|Default|GetDirectionToMove)
    (:0
      (bind _array_element (Utilities|Array|ForEachLoopwithBreak (Variables|Default|GetNormalEnemiesList) :!label _label)
        (:LoopBody
          (if (<= (.y (Transformation|GetActorLocation _array_element)) (Variables|MapSettings|GetLimitLeft))
            (for _array_element_2 (Variables|Default|GetNormalEnemiesList)
              (bind _output_get (Variables|/Game/MainFolder/Blueprints/Enemies/BP_Enemy0.BP_Enemy0_C|SetDirectionToMove _array_element_2 1))
              (Variables|Default|SetDirectionToMove _output_get))
            (goto _label Break)))))
    (:1
      (for _array_element_3 (Variables|Default|GetNormalEnemiesList)
        (if (Utilities|IsValid _array_element_3)
          (Variables|/Game/MainFolder/Blueprints/Enemies/BP_Enemy0.BP_Enemy0_C|SetDirectionToMove _array_element_3 3)))
      (Variables|Default|SetDirectionToMove 3))
    (:2
      (for _array_element_4 (Variables|Default|GetNormalEnemiesList)
        (if (Utilities|IsValid _array_element_4)
          (Variables|/Game/MainFolder/Blueprints/Enemies/BP_Enemy0.BP_Enemy0_C|SetDirectionToMove _array_element_4 0)))
      (Variables|Default|SetDirectionToMove 0))
    (:3
      (bind _array_element_5 (Utilities|Array|ForEachLoopwithBreak (Variables|Default|GetNormalEnemiesList) :!label _label_2)
        (:LoopBody
          (if (>= (.y (Transformation|GetActorLocation _array_element_5)) (Variables|MapSettings|GetLimitRight))
            (for _array_element_6 (Variables|Default|GetNormalEnemiesList)
              (bind _output_get_2 (Variables|/Game/MainFolder/Blueprints/Enemies/BP_Enemy0.BP_Enemy0_C|SetDirectionToMove _array_element_6 2))
              (Variables|Default|SetDirectionToMove _output_get_2))
            (goto _label_2 Break)))))))

(fn EndGameSuccess
  ;[1 1 1] If all enemies are dispatched, stop the logic, the player and shows the end UI
  (if (== (Variables|Default|GetInitNumEnemies) (Variables|Default|GetDeadEnemiesNum))
    (Utilities|Time|ClearandInvalidateTimerbyHandle (Variables|Default|GetSpeedTimer))
    (Utilities|Time|ClearandInvalidateTimerbyHandle (Variables|Default|GetSpecialEnemSpawnTimer))
    (Utilities|Time|ClearandInvalidateTimerbyHandle (Variables|Default|GetEnemyShootingTimer))
    (bind _asbp_player_controller (Utilities|Casting|CastToBP_PlayerController (Game|GetPlayerController 0)))
    (Variables|/Game/MainFolder/Blueprints/Player/BP_PlayerController.BP_PlayerController_C|SetEnabledInput _asbp_player_controller false)
    (Variables|/Script/Engine.MovementComponent|SetVelocity (Pawn|GetMovementComponent (Pawn|GetControlledPawn _asbp_player_controller)) "0, 0, 0")
    (bind _asbp_game_mode (Utilities|Casting|CastToBP_GameMode (Game|GetGameMode)))
    (Default|EndGame (Variables|/Game/MainFolder/Blueprints/Manager/BP_GameMode.BP_GameMode_C|GetWidgetUI _asbp_game_mode) true)))

(fn EndGameFailure
  ;[1 1 1] stop the logic, the player and shows the end UI without the completed stage message
  (Utilities|Time|ClearandInvalidateTimerbyHandle (Variables|Default|GetSpeedTimer))
  (Utilities|Time|ClearandInvalidateTimerbyHandle (Variables|Default|GetSpecialEnemSpawnTimer))
  (Utilities|Time|ClearandInvalidateTimerbyHandle (Variables|Default|GetEnemyShootingTimer))
  (bind _asbp_player_controller (Utilities|Casting|CastToBP_PlayerController (Game|GetPlayerController 0)))
  (Variables|/Game/MainFolder/Blueprints/Player/BP_PlayerController.BP_PlayerController_C|SetEnabledInput _asbp_player_controller false)
  (Variables|/Script/Engine.MovementComponent|SetVelocity (Pawn|GetMovementComponent (Pawn|GetControlledPawn _asbp_player_controller)) "0, 0, 0")
  (bind _asbp_game_mode (Utilities|Casting|CastToBP_GameMode (Game|GetGameMode)))
  (Default|EndGame (Variables|/Game/MainFolder/Blueprints/Manager/BP_GameMode.BP_GameMode_C|GetWidgetUI _asbp_game_mode) false))

(fn SpawnSpecialEnemy
  (bind _specenemstartendpos (Variables|EnemySettings|GetSpecEnemStartEndPos))
  (bind _output (Utilities|Array|Get(acopy) _specenemstartendpos))
  (bind _actorref (ObjectPooler|ObjectPoolSpawn "/Game/MainFolder/Blueprints/Enemies/BP_Enemy1.BP_Enemy1_C"))
  (bind _asbp_enemy_1 (Utilities|Casting|CastToBP_Enemy1 _actorref))
  (Variables|/Script/Engine.MovementComponent|SetVelocity (Variables|/Game/MainFolder/Blueprints/Enemies/BP_Enemy1.BP_Enemy1_C|GetProjectileMovement _asbp_enemy_1) (Math|Vector|MakeVector 0.0 (* -1 (Variables|EnemySettings|GetSpecialEnemySpeed)) 0.0))
  (Transformation|SetActorLocation _asbp_enemy_1 (Math|Vector|MakeVector (.x _output) (.y _output) (.z _output)) false false)
  (Variables|/Game/MainFolder/Blueprints/Enemies/BP_Enemy1.BP_Enemy1_C|SetAwardedPoints _asbp_enemy_1 (Variables|EnemySettings|GetSpecEnemAwardedPoints))
  (Variables|/Game/MainFolder/Blueprints/Enemies/BP_Enemy1.BP_Enemy1_C|SetLimitLeftToDespawn _asbp_enemy_1 (.y (Utilities|Array|Get(acopy) (Variables|EnemySettings|GetSpecEnemStartEndPos) 1)))
  (Rendering|SetActorHiddenInGame _asbp_enemy_1 false)
  (Actor|Tick|SetActorTickEnabled _asbp_enemy_1 true)
  (Variables|/Script/Engine.PrimitiveComponent|SetbGenerateOverlapEvents (Variables|/Game/MainFolder/Blueprints/Enemies/BP_EnemyBase.BP_EnemyBase_C|GetHitbox _asbp_enemy_1) true))

(fn EnemyShooting
  (bind _enemiesallowedtoshoot (LocalVariables|GetEnemiesAllowedToShoot))
  (bind _returnvalue (Utilities|Array|Length _enemiesallowedtoshoot))
  ;[1 1 1] 1st loop. Fills a list of the closest enemies to the bottom for each column.        2nd loop. cleans the nullptr in the list.      Select a random enemy and makes it shoot. Then empties the first list
  (for _array_element (Variables|Default|GetNormalEnemiesList)
    (if (Utilities|IsValid _array_element)
      (if (Utilities|IsValid (Utilities|Array|Get(acopy) (Variables|Default|GetEnemiesToShoot) (Variables|/Game/MainFolder/Blueprints/Enemies/BP_Enemy0.BP_Enemy0_C|GetColumn _array_element)))
        (if (< (Variables|/Game/MainFolder/Blueprints/Enemies/BP_Enemy0.BP_Enemy0_C|GetRow (Utilities|Array|Get(acopy) (Variables|Default|GetEnemiesToShoot) (Variables|/Game/MainFolder/Blueprints/Enemies/BP_Enemy0.BP_Enemy0_C|GetColumn _array_element))) (Variables|/Game/MainFolder/Blueprints/Enemies/BP_Enemy0.BP_Enemy0_C|GetRow _array_element))
          (Utilities|Array|SetArrayElem (Variables|Default|GetEnemiesToShoot) (Variables|/Game/MainFolder/Blueprints/Enemies/BP_Enemy0.BP_Enemy0_C|GetColumn _array_element) _array_element))
        (else
          (Utilities|Array|SetArrayElem (Variables|Default|GetEnemiesToShoot) (Variables|/Game/MainFolder/Blueprints/Enemies/BP_Enemy0.BP_Enemy0_C|GetColumn _array_element) _array_element)))))
  (for _array_element_2 (Variables|Default|GetEnemiesToShoot)
    (if (Utilities|IsValid _array_element_2)
      (Utilities|Array|Add (LocalVariables|GetEnemiesAllowedToShoot) _array_element_2)))
  (if (> _returnvalue 0)
    (bind _actorref (ObjectPooler|ObjectPoolSpawn "/Game/MainFolder/Blueprints/Enemies/BP_EnemyBullet.BP_EnemyBullet_C"))
    (bind _asbp_enemy_bullet (Utilities|Casting|CastToBP_EnemyBullet _actorref))
    (Variables|/Script/Engine.MovementComponent|SetVelocity (Variables|/Game/MainFolder/Blueprints/Enemies/BP_EnemyBullet.BP_EnemyBullet_C|GetProjectileMovement _asbp_enemy_bullet) (Math|Vector|MakeVector (* -1 (Variables|EnemySettings|GetEnemyBulletSpeed)) 0.0 0.0))
    (Transformation|SetActorLocation _asbp_enemy_bullet (Transformation|GetActorLocation (Utilities|Array|Get(acopy) _enemiesallowedtoshoot (Math|Random|RandomInteger (- _returnvalue 1)))) false false)
    (Rendering|SetActorHiddenInGame _asbp_enemy_bullet false)
    (Variables|/Script/Engine.PrimitiveComponent|SetbGenerateOverlapEvents (Variables|/Game/MainFolder/Blueprints/Enemies/BP_EnemyBullet.BP_EnemyBullet_C|GetHitbox _asbp_enemy_bullet) true)
    (for (_ _array_index) (Variables|Default|GetEnemiesToShoot)
      (Utilities|Array|SetArrayElem (Variables|Default|GetEnemiesToShoot) _array_index 0))))

(fn UpdateEnemyShootin
  (Utilities|Time|ClearandInvalidateTimerbyHandle (Variables|Default|GetEnemyShootingTimer))
  (Variables|Default|SetCurrentEnemyShootFreq (- (Variables|Default|GetCurrentEnemyShootFreq) (/ (- (Variables|EnemySettings|GetEnemyBaseShootFreq) (Variables|EnemySettings|GetEnemyMaxShootFreq)) (Math|Conversions|ToFloat(Integer) (Variables|Default|GetInitNumEnemies)))))
  (if (!= (Variables|Default|GetLastEnemyShootFreq) (Variables|Default|GetCurrentEnemyShootFreq))
    (EnemySettings|EnemyShooting)
    (bind _returnvalue (Utilities|Time|SetTimerbyFunctionName 0 "EnemyShooting" (Variables|Default|GetCurrentEnemyShootFreq) true))
    (Variables|Default|SetEnemyShootingTimer _returnvalue)
    (Variables|Default|SetLastEnemyShootFreq (Variables|Default|GetCurrentEnemyShootFreq))
    (else
      (Development|PrintString "Hello"))))

(fn PauseandUnPauseLogic
  (Utilities|Time|ClearandInvalidateTimerbyHandle (Variables|Default|GetSpeedTimer))
  (Utilities|Time|ClearandInvalidateTimerbyHandle (Variables|Default|GetSpecialEnemSpawnTimer))
  (Utilities|Time|ClearandInvalidateTimerbyHandle (Variables|Default|GetEnemyShootingTimer))
  (bind _returnvalue (Utilities|Time|SetTimerbyFunctionName 0 "EnemyMove" (Variables|Default|GetCurrentEnemySpeed) true 1.7))
  (Variables|Default|SetSpeedTimer _returnvalue)
  (bind _returnvalue_2 (Utilities|Time|SetTimerbyFunctionName 0 "SpawnSpecialEnemy" 2e+01 true))
  (Variables|Default|SetSpecialEnemSpawnTimer _returnvalue_2)
  (bind _returnvalue_3 (Utilities|Time|SetTimerbyFunctionName 0 "EnemyShooting" (Variables|Default|GetCurrentEnemyShootFreq) true 1.7))
  (Variables|Default|SetEnemyShootingTimer _returnvalue_3))

(fn EnemyMove
  (EnemySettings|MovebyTurn)
  ;[1 1 1] Update Speeds if an Enemy dies, if all enemies are dead, ends game
  (if (!= (Variables|Default|GetDeadEnemiesNum) (Variables|Default|GetLastDeadEnemiesNum))
    (MapSettings|EndGameSuccess)
    (Variables|Default|SetCurrentEnemySpeed (- (Variables|Default|GetCurrentEnemySpeed) (/ (- (Variables|EnemySettings|GetMinEnemySpeed) (Variables|EnemySettings|GetMaxEnemySpeed)) (Math|Conversions|ToFloat(Integer) (Variables|Default|GetInitNumEnemies)))))
    (Utilities|Time|ClearandInvalidateTimerbyHandle (Variables|Default|GetSpeedTimer))
    (bind _returnvalue (Utilities|Time|SetTimerbyFunctionName 0 "EnemyMove" (Variables|Default|GetCurrentEnemySpeed) true))
    (Variables|Default|SetSpeedTimer _returnvalue)
    (EnemySettings|UpdateEnemyShootin)
    (Variables|Default|SetLastDeadEnemiesNum (Variables|Default|GetDeadEnemiesNum)))
  (if (Variables|Default|GetChangeDirection)
    (EnemySettings|EnemyChangeDirection)))