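; Player bullet actor that kills enemies on hitbox overlap and awards their points.
; Obstacles, top-down colliders and both enemy types end the bullet; enemy hits also call the enemy's despawn and add its points.
; Despawn hides the bullet, zeroes its velocity and disables overlaps rather than destroying it.
; Score updates write straight to the GameMode's UI widget as a string zero-padded to four digits.
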(event OnComponentBeginOverlap(Hitbox)
  (params (OverlappedComponent :type Primitive%20Component%20Object%20Reference) (OtherActor :type Actor%20Object%20Reference) (OtherComp :type Primitive%20Component%20Object%20Reference) (OtherBodyIndex :type Integer) (bFromSweep :type Boolean) (SweepResult :type Hit%20Result%20Structure%20%28by%20ref%29))
  (Utilities|Casting|CastToBP_Obstacle OtherActor
    (:then
      _)
    (:CastFailed
      (Utilities|Casting|CastToBP_TopDownCollider OtherActor
        (:then
          _)
        (:CastFailed
          (bind _asbp_enemy_0 (Utilities|Casting|CastToBP_Enemy0 OtherActor)
            (:then
              (Default|SetValuesonDespawn _asbp_enemy_0)
              (CallFunction|AddScore (Variables|/Game/MainFolder/Blueprints/Enemies/BP_Enemy0.BP_Enemy0_C|GetAwardedPoints _asbp_enemy_0)))
            (:CastFailed
              (bind _asbp_enemy_1 (Utilities|Casting|CastToBP_Enemy1 OtherActor))
              (Default|SetValuesonDespawn _asbp_enemy_1)
              (CallFunction|AddScore (Variables|/Game/MainFolder/Blueprints/Enemies/BP_Enemy1.BP_Enemy1_C|GetAwardedPoints _asbp_enemy_1))))))))
  (CallFunction|OnDespawn))

(fn ConstructionScript)

(fn OnDespawn
  (Rendering|SetActorHiddenInGame true)
  (Variables|/Script/Engine.MovementComponent|SetVelocity (Variables|Default|GetProjectileMovement) "0, 0, 0")
  (Variables|/Script/Engine.PrimitiveComponent|SetbGenerateOverlapEvents (Variables|Default|GetHitbox) false))

(fn AddScore
  (params (awardedPoints :type Integer%20%28by%20ref%29))
  ;[1 1 1] Add the score of each enemy to a base string of "0000" in the UI
  (bind _asbp_game_mode (Utilities|Casting|CastToBP_GameMode (Game|GetGameMode)))
  (Variables|/Game/MainFolder/Blueprints/UI/BP_UI.BP_UI_C|SetScore (Variables|/Game/MainFolder/Blueprints/Manager/BP_GameMode.BP_GameMode_C|GetWidgetUI _asbp_game_mode) (Utilities|String|Append (Utilities|String|Right "0000" (- 4 (Utilities|String|Len (Utilities|String|ToString(Integer) (+ (Math|Conversions|ToInteger(Byte) (Variables|/Game/MainFolder/Blueprints/UI/BP_UI.BP_UI_C|GetScore (Variables|/Game/MainFolder/Blueprints/Manager/BP_GameMode.BP_GameMode_C|GetWidgetUI _asbp_game_mode))) awardedPoints))))) (Utilities|String|ToString(Integer) (+ (Math|Conversions|ToInteger(Byte) (Variables|/Game/MainFolder/Blueprints/UI/BP_UI.BP_UI_C|GetScore (Variables|/Game/MainFolder/Blueprints/Manager/BP_GameMode.BP_GameMode_C|GetWidgetUI _asbp_game_mode))) awardedPoints)))))