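; Player pawn for a shooter that fires pooled bullets along X and loses lives to enemy bullets.
; Shooting takes a BP_Bullet from the scene manager's object pool, then starts a timer cooldown.
; A hit updates the lives UI, disables input and either ends the game or triggers the manager's pause logic.
; On survival, a looping timer steps a death blink via material parameter and visibility, then restores input if enemies remain.
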(event Custom|EndCooldown
  ;[1 1 1] obtains a Bullet from the Object Pooler, sets its position and enables it. Then establish a cooldown to shoot again
  (Variables|Default|SetRecharging false)
  (Utilities|Time|ClearandInvalidateTimerbyHandle (Variables|Default|GetCooldownTimerHandle)))

(event EventBeginPlay
  (bind _returnvalue (Rendering|Material|CreateDynamicMaterialInstance (Utilities|Array|Get(acopy) (Rendering|Material|GetMaterials (Variables|Default|GetSprite))) "None" "None" :!class /Script/Engine.KismetMaterialLibrary))
  (bind _output_get (Variables|Default|SetMaterialInst _returnvalue))
  (Rendering|Material|SetMaterial (Variables|Default|GetSprite) 0 _output_get))

(event Input|ActionEvents|InputActionShoot
  (params (Key :type Key%20Structure))
  (bind _self self)
  (bind _returnvalue (Transformation|GetActorLocation _self))
  (:Pressed
    (bind _asbp_player_controller (Utilities|Casting|CastToBP_PlayerController (Game|GetPlayerController 0)))
    (if (Variables|/Game/MainFolder/Blueprints/Player/BP_PlayerController.BP_PlayerController_C|GetEnabledInput _asbp_player_controller)
      (if (not (Variables|Default|GetRecharging))
        ;[1 1 1] obtains a Bullet from the Object Pooler, sets its position and enables it. Then establish a cooldown to shoot again
        (if (Utilities|IsValid (Variables|Default|GetSceneManagerRef))
          (bind _actorref (Default|ObjectPoolSpawn (Variables|Default|GetSceneManagerRef) "/Game/MainFolder/Blueprints/Player/BP_Bullet.BP_Bullet_C"))
          (bind _asbp_bullet (Utilities|Casting|CastToBP_Bullet _actorref))
          (Variables|/Script/Engine.MovementComponent|SetVelocity (Variables|/Game/MainFolder/Blueprints/Player/BP_Bullet.BP_Bullet_C|GetProjectileMovement _asbp_bullet) (Math|Vector|MakeVector (Variables|/Game/MainFolder/Blueprints/Manager/SceneManager.SceneManager_C|GetPlayerBulletSpeed (Variables|Default|GetSceneManagerRef)) 0.0 0.0))
          (Transformation|SetActorLocation _asbp_bullet (Math|Vector|MakeVector (+ (.x _returnvalue) 1e+01) (.y _returnvalue) (.z _returnvalue)) false false)
          (Rendering|SetActorHiddenInGame _asbp_bullet false)
          (Variables|/Script/Engine.PrimitiveComponent|SetbGenerateOverlapEvents (Variables|/Game/MainFolder/Blueprints/Player/BP_Bullet.BP_Bullet_C|GetHitbox _asbp_bullet) true)
          (Variables|Default|SetRecharging true)
          (bind _returnvalue_2 (Utilities|Time|SetTimerbyEvent (delegate Custom|EndCooldown) (Variables|/Game/MainFolder/Blueprints/Manager/SceneManager.SceneManager_C|GetPlayerShootCooldown (Variables|Default|GetSceneManagerRef))))
          (Variables|Default|SetCooldownTimerHandle _returnvalue_2))))))

(fn ConstructionScript)

(fn OnHitbyEnemyBullet
  (bind _scenemanagerref (Variables|Default|GetSceneManagerRef))
  (Variables|Default|SetLives (- (Variables|Default|GetLives) 1))
  (bind _asbp_game_mode (Utilities|Casting|CastToBP_GameMode (Game|GetGameMode)))
  (Variables|/Game/MainFolder/Blueprints/UI/BP_UI.BP_UI_C|SetLives (Variables|/Game/MainFolder/Blueprints/Manager/BP_GameMode.BP_GameMode_C|GetWidgetUI _asbp_game_mode) (Variables|Default|GetLives))
  (if (<= (Variables|Default|GetLives) 0)
    (Default|EndGameFailure _scenemanagerref)
    (bind _asbp_player_controller (Utilities|Casting|CastToBP_PlayerController (Game|GetPlayerController 0)))
    (Variables|/Game/MainFolder/Blueprints/Player/BP_PlayerController.BP_PlayerController_C|SetEnabledInput _asbp_player_controller false)
    (Variables|/Script/Engine.MovementComponent|SetVelocity (Pawn|GetMovementComponent) "0, 0, 0")
    (else
      (Default|PauseandUnPauseLogic _scenemanagerref)
      (bind _asbp_player_controller_2 (Utilities|Casting|CastToBP_PlayerController (Game|GetPlayerController 0)))
      (Variables|/Game/MainFolder/Blueprints/Player/BP_PlayerController.BP_PlayerController_C|SetEnabledInput _asbp_player_controller_2 false)
      (Variables|/Script/Engine.MovementComponent|SetVelocity (Pawn|GetMovementComponent) "0, 0, 0")
      (bind _returnvalue (Utilities|Time|SetTimerbyFunctionName 0 "DelayToReturnImputs" 0.425 true))
      (Variables|Default|SetRespawnTimer _returnvalue))))

(fn DelaytoReturnImputs
  (bind _scenemanagerref (Variables|Default|GetSceneManagerRef))
  (bind _output_get (Variables|Default|SetSpriteAnimState (+ (Variables|Default|GetSpriteAnimState) 1)))
  (CallFunction|PlayerDeathAnim _output_get)
  (if (== (Variables|Default|GetSpriteAnimState) 4)
    (Utilities|Time|ClearandInvalidateTimerbyHandle (Variables|Default|GetRespawnTimer))
    (Variables|Default|SetSpriteAnimState 0)
    (if (not (== (Variables|/Game/MainFolder/Blueprints/Manager/SceneManager.SceneManager_C|GetInitNumEnemies _scenemanagerref) (Variables|/Game/MainFolder/Blueprints/Manager/SceneManager.SceneManager_C|GetDeadEnemiesNum _scenemanagerref)))
      (bind _asbp_player_controller (Utilities|Casting|CastToBP_PlayerController (Game|GetPlayerController 0)))
      (Variables|/Game/MainFolder/Blueprints/Player/BP_PlayerController.BP_PlayerController_C|SetEnabledInput _asbp_player_controller true))))

(fn PlayerDeathAnim
  (params (StateOfPlayer :type Integer%20%28by%20ref%29))
  (switch int StateOfPlayer
    (:1
      (Rendering|Material|SetScalarParameterValue (Variables|Default|GetMaterialInst) "Tex01" 1.0 :!class /Script/Engine.MaterialInstanceDynamic)
      (Rendering|SetVisibility (Variables|Default|GetSprite) true false))
    (:2
      (Rendering|SetVisibility (Variables|Default|GetSprite) false false))
    (:3
      (Rendering|Material|SetScalarParameterValue (Variables|Default|GetMaterialInst) "Tex01" 0.0 :!class /Script/Engine.MaterialInstanceDynamic)
      (Rendering|SetVisibility (Variables|Default|GetSprite) true false))))