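; BP_PlayerController moves the player pawn left and right along world Y between two limits.
; The MoveRightLeft axis, gated by EnabledInput, caches the pawn's movement component and sets its velocity directly from the axis value times Velocity.
; A switch on the truncated axis zeroes velocity at the limit in the direction of travel, so fractional input skips the limit check.
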(event Input|AxisEvents|InputAxisMoveRightLeft
  (params (AxisValue :type Float%20%28single-precision%29))
  (if (Variables|Default|GetEnabledInput)
    (Variables|Default|SetAxisval AxisValue)
    (if (Utilities|IsValid (Variables|Default|GetPlayerPawn))
      (if (Utilities|IsValid (Variables|Default|GetMovCompo))
        _
        (else
          (Variables|Default|SetMovCompo (Pawn|GetMovementComponent (Variables|Default|GetPlayerPawn)))))
      (switch int (Math|Float|Truncate (Variables|Default|GetAxisval))
        (:-1
          (if (>= (Variables|Default|GetLimitLeft) (.y (Transformation|GetActorLocation (Variables|Default|GetPlayerPawn))))
            (Variables|/Script/Engine.MovementComponent|SetVelocity (Variables|Default|GetMovCompo) (Math|Vector|MakeVector 0.0 0.0 0.0))
            (else
              (Variables|/Script/Engine.MovementComponent|SetVelocity (Variables|Default|GetMovCompo) (Math|Vector|MakeVector 0.0 (* (Variables|Default|GetAxisval) (Variables|Default|GetVelocity)) 0.0) :!label _label))))
        (:0
          (goto _label))
        (:1
          (if (<= (Variables|Default|GetLimitRight) (.y (Transformation|GetActorLocation (Variables|Default|GetPlayerPawn))))
            (Variables|/Script/Engine.MovementComponent|SetVelocity (Variables|Default|GetMovCompo) (Math|Vector|MakeVector 0.0 0.0 0.0))
            (else
              (goto _label))))))))

(fn ConstructionScript)